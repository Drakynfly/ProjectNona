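; Player controller that turns MIDI device input into a polyphonic synth tuned to a custom "Nona" scale of eight notes per nona.
; At BeginPlay it flattens the Nonas data table into an indexed frequency map, looked up by offset MIDI note.
; Each note spawns a MetaSound with that frequency and velocity-based volume, tracked until note-off.
; Pitch bend retunes held sounds; an output device can be selected but receives no messages here.
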(event `self.ReceiveBeginPlay`
  (set `self.bShowMouseCursor` true)
  (`self.TabulateNonaFrequencies`))

(event `HandleMidiNoteOn`
  (params (MIDIDeviceController :type "MIDIDeviceInputController Object Reference") (Timestamp :type Integer) (Channel :type Integer) (Note :type Integer) (Velocity :type Integer))
  (`KismetSystemLibrary.PrintString` (`KismetTextLibrary.Conv_TextToString` (`|FormatText` "Device: {dev} \nTime: {time} \nChannel: {chan} \nNote: {note} \nVel: {vel}" (`MIDIDeviceInputController.DeviceName` MIDIDeviceController) Timestamp Channel Note Velocity)) true true (struct :`G` 0.66 :`B` 1.0 :`A` 1.0) 2.0 "Note")
  (bind _returnvalue (`GameplayStatics.CreateSound2D` "/Game/Blueprints/MSS_Midi.MSS_Midi" (`self.VelocityToVolume` Velocity) (`self.Pitch`) 0.0 null false false))
  (`AudioComponent.Play` _returnvalue 0.0)
  (bind _frequency (`self.MIDINoteToNonaFrequency` Note))
  (`AudioComponent.SetFloatParameter` _returnvalue "Frequency" _frequency)
  (`BlueprintMapLibrary.Map_Add` (`self.ConcurrentNotes`) Note _returnvalue))

(event `SetInputDevice`
  (params (DeviceID :type Integer))
  (`self.DisableInputDevice`)
  (bind _returnvalue (`MIDIDeviceManager.CreateMIDIDeviceInputController` DeviceID))
  (bind _output_get (set `self.InMidi` _returnvalue))
  (add `MIDIDeviceInputController.OnMIDINoteOn` _output_get (`|CreateDelegate` :!event `HandleMidiNoteOn`))
  (add `MIDIDeviceInputController.OnMIDINoteOff` _output_get (`|CreateDelegate` :!event `HandleMidiNoteOff`))
  (add `MIDIDeviceInputController.OnMIDIPitchBend` _output_get (`|CreateDelegate` :!event `ChangePitchModulation`)))

(event `HandleMidiNoteOff`
  (params (MIDIDeviceController :type "MIDIDeviceInputController Object Reference") (Timestamp :type Integer) (Channel :type Integer) (Note :type Integer) (Velocity :type Integer))
  (bind _concurrentnotes (`self.ConcurrentNotes`))
  (bind _value (`BlueprintMapLibrary.Map_Find` _concurrentnotes Note))
  (`AudioComponent.Stop` _value)
  (`ActorComponent.K2_DestroyComponent` _value)
  (`BlueprintMapLibrary.Map_Remove` _concurrentnotes Note))

(event `SetOutputDevice`
  (params (DeviceID :type Integer))
  (`self.DisableOutputDevice`)
  (`KismetSystemLibrary.PrintString` (`KismetStringLibrary.Concat_StrStr` "Trying to connect to Output: " (`KismetStringLibrary.Conv_IntToString` DeviceID)))
  (bind _returnvalue (`MIDIDeviceManager.CreateMIDIDeviceOutputController` DeviceID))
  (bind _output_get (set `self.OutMidi` _returnvalue))
  (`/Engine/EditorBlueprintResources/StandardMacros.IsValid` _output_get
    (:`Is Valid`
      (`KismetSystemLibrary.PrintString` "Connection Success"))
    (:`Is Not Valid`
      (`KismetSystemLibrary.PrintString` "Connection Failed"))))

(event `ChangePitchModulation`
  (params (MIDIDeviceController :type "MIDIDeviceInputController Object Reference") (Timestamp :type Integer) (Channel :type Integer) (Pitch :type Integer))
  ;[1 1 1] Pitch Modulation
  (bind _output_get (set `self.Pitch` (`KismetMathLibrary.MapRangeClamped` (`KismetMathLibrary.Conv_IntToDouble` Pitch) 0.0 16383.0 0.0 2.0)))
  (`KismetSystemLibrary.PrintString` (`KismetStringLibrary.Conv_DoubleToString` _output_get) true true (struct :`R` 0.17482 :`G` 1.0 :`A` 1.0) 5.0 "Pitch")
  (`self.UpdatePitch`))

(event `DisableInputDevice`
  (bind _inmidi (`self.InMidi`)
    (:`then`
      (clear `MIDIDeviceInputController.OnMIDINoteOn` _inmidi)
      (clear `MIDIDeviceInputController.OnMIDINoteOff` _inmidi)
      (set `self.InMidi` null))
    (:`else`)))

(event `DisableOutputDevice`
  (set `self.OutMidi` null))

(event `UpdatePitch`
  ;[1 1 1] Pitch Modulation
  (bind _values (`BlueprintMapLibrary.Map_Values` (`self.ConcurrentNotes`)))
  (for _array_element _values
    (`AudioComponent.SetPitchMultiplier` _array_element (`self.Pitch`))))

(fn `GetNonaFrequencies`
  (params (NewParam :type "/Game/Data/ENonas Enum" :default "NewEnumerator0"))
  (returns (Frequencies :type "/Game/Blueprints/FNonaFrequencies Structure"))
  (bind _returnvalue (`|GetDataTableRow` (`self.Nonas`) (`KismetStringLibrary.Conv_StringToName` (`|GetEnumeratorNameAsString` NewParam)))
    (:`then`
      (return _returnvalue))
    (:`RowNotFound`
      (`KismetSystemLibrary.PrintString` "BadRow")
      (return))))

(fn `MIDINoteToNonaFrequency`
  (params (Note :type Integer))
  (returns (Frequency :type "Float (double-precision)"))
  (bind _value (`BlueprintMapLibrary.Map_Find` (`self.NonaFrequencies`) (+ Note (`self.MidiNoteOffset`))))
  (`KismetSystemLibrary.PrintString` (`KismetStringLibrary.Conv_DoubleToString` _value))
  (return _value))

(fn `TabulateNonaFrequencies`
  (locals (L_NonaIndex :type Integer))
  (bind _l_nonaindex (`local.L_NonaIndex`))
  (bind _enumvalue (foreach `/Game/Data/ENonas` true)
    (:`LoopBody`
      (bind _enumvalue_2 (foreach `/Game/Data/ENonaNote` true)
        (:`LoopBody`
          (bind (_e _f _g _h _a _b _c _d) (break `/Game/Blueprints/FNonaFrequencies` (`self.GetNonaFrequencies` _enumvalue)))
          (bind _returnvalue (select `/Game/Data/ENonaNote` _enumvalue_2 :`NewEnumerator0` _e :`NewEnumerator1` _f :`NewEnumerator2` _g :`NewEnumerator3` _h :`NewEnumerator4` _a :`NewEnumerator5` _b :`NewEnumerator6` _c :`NewEnumerator7` _d))
          (`BlueprintMapLibrary.Map_Add` (`self.NonaFrequencies`) _l_nonaindex _returnvalue)
          (`/Engine/EditorBlueprintResources/StandardMacros.IncrementInt` (`local.L_NonaIndex`)
            (:`  `
              (`KismetSystemLibrary.PrintString` (`KismetStringLibrary.Concat_StrStr` (`KismetStringLibrary.Conv_DoubleToString` _returnvalue) " = " (`KismetStringLibrary.Conv_IntToString` _l_nonaindex))))))))
    (:`then`
      (return))))

(fn `UserConstructionScript`)

(fn `VelocityToVolume`
  (params (Velocity :type Integer))
  (returns (Volume :type "Float (double-precision)"))
  (return (`KismetMathLibrary.MapRangeClamped` (`KismetMathLibrary.Conv_IntToDouble` Velocity) 0.0 127.0 0.0 1.0)))